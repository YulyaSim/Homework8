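; Grid of breakable blocks that take two hits from BP_Actor_Sphere and can drop a random bonus actor.
; The construction script builds the grid as static mesh components on this one actor, spaced by Padding.
; On Hit, the chrome material doubles as damage state: a non-chrome block turns chrome, while a chrome block is destroyed, with a coin-flip chance to spawn an actor above it.
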(event `self.ReceiveBeginPlay`)

(event `self.ReceiveTick`
  (params (DeltaSeconds :type "Float (single-precision)")))

(event `self.ReceiveHit`
  (params (MyComp :type "PrimitiveComponent Object Reference") (Other :type "Actor Object Reference") (OtherComp :type "PrimitiveComponent Object Reference") (bSelfMoved :type Boolean) (HitLocation :type "Vector Structure") (HitNormal :type "Vector Structure") (NormalImpulse :type "Vector Structure") (Hit :type "HitResult Structure (by ref)"))
  (bind _returnvalue (`KismetMathLibrary.Conv_VectorToTransform` (`SceneComponent.K2_GetComponentLocation` MyComp)))
  (cast `/Game/BP_Actor_Sphere` Other)
  (bind _asstatic_mesh_component (cast `StaticMeshComponent` MyComp))
  (if (== (`|GetArrayItem` (`MeshComponent.GetMaterials` _asstatic_mesh_component)) "/Game/StarterContent/Materials/M_Metal_Chrome.M_Metal_Chrome")
    (if (`KismetMathLibrary.RandomBoolWithWeight` 0.5)
      (`|SpawnActorFromClass` (`|GetArrayItem` (`self.Class`) (`KismetMathLibrary.RandomIntegerInRange` 0 2)) (`KismetMathLibrary.MakeTransform` (`KismetMathLibrary.MakeVector` (.x (.location _returnvalue)) (.y (.location _returnvalue)) (+ (.z (.location _returnvalue)) 60.0)) (.rotation _returnvalue) (.scale _returnvalue)) "AlwaysSpawn" "OverrideRootScale" null null))
    (`ActorComponent.K2_DestroyComponent` MyComp)
    (`KismetSystemLibrary.PrintString` "Destroy" true true (struct :`R` 0.345274 :`G` 1.0 :`A` 1.0))
    (else
      (`PrimitiveComponent.SetMaterial` _asstatic_mesh_component 0 "/Game/StarterContent/Materials/M_Metal_Chrome.M_Metal_Chrome")
      (`KismetSystemLibrary.PrintString` "Change Color" true true (struct :`R` 1.0 :`G` 0.75 :`A` 1.0)))))

(fn `UserConstructionScript`
  (for _index (range (+ (`self.X`) 1))
    (for _index_2 (range (+ (`self.Y`) 1))
      (`AddComponent|NODE_AddStaticMeshComponent-0` :`RelativeTransform` (`KismetMathLibrary.MakeTransform` (`KismetMathLibrary.MakeVector` (`KismetMathLibrary.Conv_IntToDouble` (* _index (`self.Padding`))) (`KismetMathLibrary.Conv_IntToDouble` (* _index_2 (`self.Padding`)))))))))