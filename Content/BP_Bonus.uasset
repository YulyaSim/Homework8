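; BP_Bonus is a bonus actor that moves through the level until it enters a kill volume.
; Tick applies a swept world offset from its direction and speed, scaled by delta time, but takes no action on blocking hits.
; Overlapping a KillZVolume destroys the actor and prints a debug message.
; A reflection-vector calculation using the hit normal is present but unused, so it never bounces.
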(event `self.ReceiveBeginPlay`)

(event `self.ReceiveDestroyed`)

(event `self.ReceiveActorBeginOverlap`
  (params (OtherActor :type "Actor Object Reference"))
  (cast `KillZVolume` OtherActor)
  (`self.K2_DestroyActor`)
  (`KismetSystemLibrary.PrintString` "Bonus Dead"))

(event `self.ReceiveTick`
  (params (DeltaSeconds :type "Float (single-precision)"))
  (bind _sweephitresult (`self.K2_AddActorWorldOffset` (* (* (`self.Bonus_Direction`) (`self.Bonus_Speed`)) DeltaSeconds) true))
  (if (`GameplayStatics.BreakHitResult` _sweephitresult)
    _))

(fn `UserConstructionScript`)