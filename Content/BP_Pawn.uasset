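; Player pawn that moves sideways and manages lives for a ball game, spawning balls at its capsule.
; MoveRight input applies fixed, swept world offsets along Y, not scaled by axis value or frame time.
; SpawnBall spends a life and, unless none remain, spawns a BP_Actor_Sphere and binds to its OnDead event.
; BeginPlay adds one life before the first spawn to offset that decrement.
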(event `InputAxis|MoveRight`
  (params (AxisValue :type "Float (single-precision)"))
  (if (< AxisValue 0.0)
    (`self.K2_AddActorWorldOffset` (0.0 50.0 0.0) true)))

(event `InputAxis|MoveRight`
  (params (AxisValue :type "Float (single-precision)"))
  (if (> AxisValue 0.0)
    (`self.K2_AddActorWorldOffset` (0.0 -50.0 0.0) true)))

(event `self.ReceiveBeginPlay`
  (set `self.Lives` (+ (`self.Lives`) 1))
  (`self.Spawn Ball`))

(fn `Spawn Ball`
  (bind _output_get (set `self.Lives` (- (`self.Lives`) 1)))
  (if (not (== _output_get 0))
    (bind _returnvalue (`|SpawnActorFromClass` "/Game/BP_Actor_Sphere.BP_Actor_Sphere_C" (`KismetMathLibrary.MakeTransform` (`SceneComponent.K2_GetComponentLocation` (`self.Capsule`))) "Undefined" "OverrideRootScale" null null))
    (bind _output_get_2 (set `self.ActorSphere` _returnvalue))
    (add `/Game/BP_Actor_Sphere.OnDead` _output_get_2 (`|CreateDelegate` :!event `Spawn Ball`))
    (return)))

(fn `UserConstructionScript`)