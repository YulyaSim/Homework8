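; BP_Bonus_SpeedUp is a bonus pickup that speeds up the BP_Actor_Sphere actors in the level.
; On overlap it runs the parent's handler, then finds every BP_Actor_Sphere, doubles its Speed and destroys itself.
; It does not check which actor overlapped, and it has no timer to revert the boost.
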(event `self.ReceiveActorBeginOverlap`
  (params (OtherActor :type "Actor Object Reference"))
  (`parent.ReceiveActorBeginOverlap` OtherActor)
  (bind _outactors (`GameplayStatics.GetAllActorsOfClass` "/Game/BP_Actor_Sphere.BP_Actor_Sphere_C"))
  (for _array_element _outactors
    (set `/Game/BP_Actor_Sphere.Speed` (* (`/Game/BP_Actor_Sphere.Speed` _array_element) 2.0) _array_element))
  (`self.K2_DestroyActor`))

(fn `UserConstructionScript`
  (`parent.UserConstructionScript`))