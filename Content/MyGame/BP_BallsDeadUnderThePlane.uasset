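; BP_BallsDeadUnderThePlane is a functional test that checks where the ball is when it dies relative to the player's paddle-like pawn.
; PrepareTest caches the BP_Pawn cube's world location and its ActorSphere, then binds to that sphere's OnDead event.
; On death, it finishes with Default if the sphere's X is below the cached cube X, otherwise with Failed.
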(event `self.ReceivePrepareTest`
  (bind _asbp_pawn (cast `/Game/BP_Pawn` (`GameplayStatics.GetPlayerPawn` 0)))
  (set `self.PawnLocation` (`SceneComponent.K2_GetComponentLocation` (`/Game/BP_Pawn.Cube` _asbp_pawn)))
  (bind _actorsphere (`/Game/BP_Pawn.ActorSphere` _asbp_pawn))
  (set `self.Sphere` _actorsphere)
  (add `/Game/BP_Actor_Sphere.OnDead` _actorsphere (delegate `OnDeadReaction`)))

(event `OnDeadReaction`
  (bind _pawnlocation_x (`KismetMathLibrary.BreakVector` (`self.PawnLocation`)))
  (bind _returnvalue_x (`KismetMathLibrary.BreakVector` (`SceneComponent.K2_GetComponentLocation` (`/Game/BP_Actor_Sphere.Sphere` (`self.Sphere`)))))
  (if (< _returnvalue_x _pawnlocation_x)
    (`self.FinishTest` "Default")
    (else
      (`self.FinishTest` "Failed"))))

(fn `UserConstructionScript`)